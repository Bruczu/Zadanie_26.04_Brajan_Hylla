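; Trampoline platform actor whose shape is built in the construction script, with no bounce logic in its event graph.
; The Top component takes its world scale from per-axis variables.
; The Bottom instanced mesh component stacks instances downward at 100-unit intervals, with the count derived from the length of the BottomEndLength vector.
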(event EventBeginPlay)

(event Collision|EventActorBeginOverlap
  (params (OtherActor :type Actor%20Object%20Reference)))

(event EventTick
  (params (DeltaSeconds :type Float%20%28single-precision%29)))

(fn ConstructionScript
  (Transformation|SetWorldScale3D (Variables|Default|GetTop) (Math|Vector|MakeVector (Variables|Trampolina|GetTop_X_Scale) (Variables|Trampolina|GetTop_Y_Scale) (Variables|Trampolina|GetTop_Z_Scale)))
  (Components|InstancedStaticMesh|AddInstance (Variables|Default|GetBottom) (Math|Transform|MakeTransform "0, 0, 0" "0, 0, 0" "1.000000,1.000000,1.000000") false)
  (for _index (range 0 (Math|Float|Truncate (/ (Math|Vector|VectorLength (Variables|Trampolina|GetBottomEndLength)) 1e+02)))
    (Components|InstancedStaticMesh|AddInstance (Variables|Default|GetBottom) (Math|Transform|MakeTransform (Math|Vector|MakeVector 0.0 0.0 (Math|Conversions|ToFloat(Integer) (* _index -100))) "0, 0, 0" "1.000000,1.000000,1.000000") false)))